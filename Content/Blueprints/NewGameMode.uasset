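; Game mode that periodically reports the online player count to the game's ChatterNew actors.
; BeginPlay starts a custom Return event that re-calls itself after a three-second Delay, forming an endless polling loop.
; Each pass finds all ChatterNew actors, passes GetNumPlayers to each valid one through GetOnlinePlayers, and prints the count.
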(event Custom|Return
  (params (Condition :type Boolean))
  (if Condition
    (Utilities|FlowControl|Delay 3.0)
    (bind _outactors (Actor|GetAllActorsOfClass "/Game/ChatterNew.ChatterNew_C"))
    (for _array_element _outactors
      (Utilities|IsValid _array_element
        (:Is%20Valid
          (bind _returnvalue (Class|GameModeBase|GetNumPlayers))
          (Default|GetOnlinePlayers _array_element _returnvalue))))
    (bind _returnvalue_2 (Class|GameModeBase|GetNumPlayers))
    (Development|PrintString (Utilities|String|Append "Online:  " (Utilities|String|ToString(Integer) _returnvalue_2)))
    (CallFunction|Return true)))

(event EventBeginPlay
  (CallFunction|Return true))

(fn ConstructionScript)